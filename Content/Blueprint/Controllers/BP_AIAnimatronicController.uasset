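; AI controller for animatronic pawns in a night game mode, driving their state updates.
; On BeginPlay it binds to the night game mode's animatronic update event and calls UpdateState on its controlled BP_AnimatronicBase each time it fires.
; When that animatronic signals path completion, the controller unbinds from the update event, so it stops advancing the pawn's state.
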(event `self.ReceiveBeginPlay`
  ;[1 1 1] Event bind setup
  (bind _asbp_night_game_mode_base (cast `/Game/Blueprint/GameModes/BP_NightGameModeBase` (`GameplayStatics.GetGameMode`)))
  (add `NightGameModeBase.OnAnimatronicUpdate` _asbp_night_game_mode_base (delegate `OnAnimatronicUpdate_Event`))
  ;[1 1 1] Unbind event on animatronic path completion
  (bind _asbp_animatronic_base (cast `/Game/Blueprint/Animatronics/BP_AnimatronicBase` (`self.K2_GetPawn`)))
  (add `AnimatronicBase.OnAnimatronicPathCompletion` _asbp_animatronic_base (delegate `OnAnimatronicPathCompletion_Event`)))

(event `OnAnimatronicUpdate_Event`
  ;[1 1 1] Event bind setup
  (bind _asbp_animatronic_base (cast `/Game/Blueprint/Animatronics/BP_AnimatronicBase` (`self.K2_GetPawn`)))
  (`/Game/Blueprint/Animatronics/BP_AnimatronicBase.UpdateState` _asbp_animatronic_base))

(event `OnAnimatronicPathCompletion_Event`
  ;[1 1 1] Unbind event on animatronic path completion
  (remove `NightGameModeBase.OnAnimatronicUpdate` (stale `self.ReceiveBeginPlay` _asbp_night_game_mode_base) (delegate `OnAnimatronicUpdate_Event`)))

(fn `UserConstructionScript`)