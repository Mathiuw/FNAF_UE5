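; Player controller for the guard in a night game mode, handling the HUD and the response to a power outage.
; On BeginPlay it creates the HUD widget and binds to the night game mode's power-out event.
; When power fails it disables click events, removes all widgets and switches back to the guard if another pawn is controlled, printing debug messages along the way.
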(event `self.ReceiveBeginPlay`
  (bind _returnvalue (`|CreateWidget` "/Game/UI/WBP_HUD.WBP_HUD_C"))
  (`UserWidget.AddToViewport` _returnvalue 0)
  (bind _asnight_game_mode_base (cast `NightGameModeBase` (`GameplayStatics.GetGameMode`)))
  (add `NightGameModeBase.OnPowerOut` _asnight_game_mode_base (delegate `OnPowerOutController`)))

(event `OnPowerOutController`
  (set `self.bEnableClickEvents` false)
  (`KismetSystemLibrary.PrintString` "Disabled controller click events" true true (struct :`R` 0.65 :`A` 1.0) 10.0)
  (`WidgetLayoutLibrary.RemoveAllWidgets`)
  (`KismetSystemLibrary.PrintString` "Removed all widgets" true true (struct :`R` 0.65 :`A` 1.0) 10.0)
  (cast `GuardBase` (`self.K2_GetPawn`)
    (:`CastFailed`
      (`self.SwitchCameraGuard`)
      (`KismetSystemLibrary.PrintString` "Returned to Guard" true true (struct :`R` 0.65 :`A` 1.0) 10.0))))

(fn `UserConstructionScript`)