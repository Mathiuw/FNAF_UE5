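; Base animatronic Blueprint that moves an enemy through a graph of states shown by looping level sequences and can end the night game.
; UpdateState rolls 1–20 against AILevel; a pass either jumpscares and completes the path at an open door on trigger states, or advances to a random next state.
; State changes stop all sequences before looping a random one.
; BeginPlay starts state 0 and binds path completion to the game mode's EndGame.
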(event `self.ReceiveBeginPlay`
  ;[1 1 1] Set event to end game OnAnimatronicPathCompletion
  (add `self.OnAnimatronicPathCompletion` (delegate `CustomEvent`))
  ;[1 1 1] State setup
  (`self.PlayStateFromIndex` 0))

(event `CustomEvent`
  ;[1 1 1] Set event to end game OnAnimatronicPathCompletion
  (bind _asnight_game_mode_base (cast `NightGameModeBase` (`GameplayStatics.GetGameMode`))
    (:`then`
      (`NightGameModeBase.EndGame` _asnight_game_mode_base))
    (:`CastFailed`
      (`KismetSystemLibrary.PrintString` "Failed cast to NightGameMode" true true (struct :`R` 0.76 :`A` 1.0) 5.0))))

(fn `PlayJumpscare`
  (`self.StopPlayingAllStates`)
  (`MovieSceneSequencePlayer.Play` (`LevelSequenceActor.SequencePlayer` (`self.Jumpscare`))))

(fn `PlayStateFromIndex`
  (params (Index :type Integer) (VariationIndex :type Integer))
  (bind _states (`self.States`))
  (if (`KismetArrayLibrary.Array_IsValidIndex` _states Index)
    (`self.PlayStateSequence` (`KismetArrayLibrary.Array_Random` (`.Sequences_28_C783289745F5BBC6D71847916CCA84C5` (break `/Game/Blueprint/Animatronics/Animatronic_State` (`|GetArrayItem` _states Index)))))
    (else
      (`KismetSystemLibrary.PrintString` "Cant play the state" true true (struct :`R` 0.97 :`A` 1.0) 5.0))))

(fn `PlayStateSequence`
  (params (`Sequence Actor` :type "LevelSequenceActor Object Reference"))
  (`self.StopPlayingAllStates`)
  (`MovieSceneSequencePlayer.PlayLooping` (`LevelSequenceActor.SequencePlayer` `Sequence Actor`) -1))

(fn `StopPlayingAllStates`
  (for _array_element (`self.States`)
    (for _array_element_2 (`.Sequences_28_C783289745F5BBC6D71847916CCA84C5` (break `/Game/Blueprint/Animatronics/Animatronic_State` _array_element))
      (`MovieSceneSequencePlayer.Stop` (`LevelSequenceActor.SequencePlayer` _array_element_2))))
  (`KismetSystemLibrary.PrintString` "Stopped playing all states" false))

(fn `UpdateState`
  (bind (_sequences _nextindexes _door _triggerjumpscare) (break `/Game/Blueprint/Animatronics/Animatronic_State` (`|GetArrayItem` (`self.States`) (`self.Index`))))
  (if (<= (`KismetMathLibrary.RandomIntegerInRange` 1 20) (`self.AILevel`))
    (`KismetSystemLibrary.PrintString` "RNG Pass" true true (struct :`R` 0.013145 :`G` 1.0 :`A` 1.0))
    (`/Engine/EditorBlueprintResources/StandardMacros.IsValid` _door
      (:`Is Valid`
        (if (and (not (`DoorBase.IsClosed` _door)) _triggerjumpscare)
          (`MovieSceneSequencePlayer.Play` (`LevelSequenceActor.SequencePlayer` (`self.Jumpscare`)))
          (`self.CompletePath`)
          (else
            (`KismetSystemLibrary.PrintString` "Door closed" true true (struct :`R` 0.013145 :`G` 1.0 :`A` 1.0))
            (bind _output_get (set `self.Index` (`KismetArrayLibrary.Array_Random` _nextindexes) :!label _label))
            (`self.PlayStateSequence` (`KismetArrayLibrary.Array_Random` (`.Sequences_28_C783289745F5BBC6D71847916CCA84C5` (break `/Game/Blueprint/Animatronics/Animatronic_State` (`|GetArrayItem` (`self.States`) _output_get))))))))
      (:`Is Not Valid`
        (goto _label)))
    (else
      (`KismetSystemLibrary.PrintString` "RNG Failed" true true (struct :`R` 0.97 :`A` 1.0)))))

(fn `UserConstructionScript`)