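; BP_GuardController is the guard's controller for the night game mode, handling the HUD and the response to a power outage.
; On BeginPlay it adds a BP_BaseWidget to the viewport and binds to BP_NightGameMode's OnPowerOut event.
; When power goes out, it disables click events, removes all widgets, and calls SwitchCameraGuard if the controlled pawn is not the Guard.
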(event `self.ReceiveBeginPlay`
  (bind _returnvalue (`|CreateWidget` "/Game/UI/BP_BaseWidget.BP_BaseWidget_C"))
  (`UserWidget.AddToViewport` _returnvalue 0)
  (bind _asbp_night_game_mode (cast `/Game/Blueprints/BP_NightGameMode` (`GameplayStatics.GetGameMode`)))
  (add `/Game/Blueprints/BP_NightGameMode.OnPowerOut` _asbp_night_game_mode (delegate `OnPowerOutController`)))

(event `OnPowerOutController`
  (set `self.bEnableClickEvents` false)
  (`WidgetLayoutLibrary.RemoveAllWidgets`)
  (cast `Guard` (`self.K2_GetPawn`)
    (:`then`
      _)
    (:`CastFailed`
      (`self.SwitchCameraGuard`)))
  (`KismetSystemLibrary.PrintString` "DISABLED CONTROLLER CLICK EVENTS AND REMOVED WIDGETS" true true (struct :`R` 0.65 :`A` 1.0)))

(fn `UserConstructionScript`)