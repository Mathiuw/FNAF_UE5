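; AI controller for animatronic pawns that drives their behavior during a night.
; On BeginPlay it binds to the NightGameMode's OnAnimatronicUpdate dispatcher.
; Each update runs the BT_AnimatronicStateUpdate behavior tree, provided the controlled BP_AnimatronicBase has states, and prints a debug message otherwise.
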(event `self.ReceiveBeginPlay`
  (bind _asnight_game_mode (cast `NightGameMode` (`GameplayStatics.GetGameMode`)))
  (add `NightGameMode.OnAnimatronicUpdate` _asnight_game_mode (delegate `OnAnimatronicUpdateHandler`)))

(event `OnAnimatronicUpdateHandler`
  (`self.CallBehaviorTree`))

(fn `CallBehaviorTree`
  (bind _asbp_animatronic_base (cast `/Game/Blueprints/Animatronics/BP_AnimatronicBase` (`self.K2_GetPawn`))
    (:`then`
      (if (== (`KismetArrayLibrary.Array_Length` (`/Game/Blueprints/Animatronics/BP_AnimatronicBase.States` _asbp_animatronic_base)) 0)
        (`KismetSystemLibrary.PrintString` "Animatronic has no states" true true (struct :`R` 0.97 :`A` 1.0))
        (else
          (`self.RunBehaviorTree` "/Game/AI/BT_AnimatronicStateUpdate.BT_AnimatronicStateUpdate"))))
    (:`CastFailed`
      (`KismetSystemLibrary.PrintString` "Cast to BP_Animatronic failed" true true (struct :`R` 0.97 :`A` 1.0) 5.0))))

(fn `UserConstructionScript`)