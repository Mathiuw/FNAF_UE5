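; Game mode base that records the current level as the restart level and handles game over.
; On BeginPlay it loads or creates the BP_Save in slot Save_1, stores the current level name in it and saves.
; It also binds to an OnGameOver event, which opens the GameOver level after a short delay.
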(event `self.ReceiveBeginPlay`
  ;[1 1 1] Save
  (`self.SaveInitialization`)
  ;[1 1 1] Game over event
  (add `self.OnGameOver` (delegate `CustomEvent`)))

(event `CustomEvent`
  ;[1 1 1] Game over event
  (`KismetSystemLibrary.Delay` 2.0)
  (`GameplayStatics.OpenLevelBySoftObjectPtr` "/Game/Levels/GameOver.GameOver"))

(fn `SaveInitialization`
  (locals (LevelName :type String))
  (bind _levelname (`local.LevelName`))
  (bind _returnvalue (`GameplayStatics.GetCurrentLevelName` true))
  (set `local.LevelName` _returnvalue)
  (bind _returnvalue_2 (`GameplayStatics.DoesSaveGameExist` "Save_1"))
  (if _returnvalue_2
    (bind _returnvalue_3 (`GameplayStatics.LoadGameFromSlot` "Save_1"))
    (bind _asbp_save (cast `/Game/Blueprints/BP_Save` _returnvalue_3)
      (:`then`
        (set `/Game/Blueprints/BP_Save.LevelRestartName` _levelname _asbp_save)
        (`GameplayStatics.SaveGameToSlot` _asbp_save "Save_1")
        (`KismetSystemLibrary.PrintString` "Game Saved" true true (struct :`R` 0.087397 :`G` 0.58 :`A` 1.0) 5.0 :!label _label))
      (:`CastFailed`
        (`KismetSystemLibrary.PrintString` "Cast to BP_Save Failed" true true (struct :`G` 0.66 :`B` 1.0 :`A` 1.0) 10.0)))
    (else
      (bind _returnvalue_4 (`GameplayStatics.CreateSaveGameObject` "/Game/Blueprints/BP_Save.BP_Save_C"))
      (set `/Game/Blueprints/BP_Save.LevelRestartName` _levelname _returnvalue_4)
      (`GameplayStatics.SaveGameToSlot` _returnvalue_4 "Save_1")
      (goto _label))))

(fn `UserConstructionScript`)